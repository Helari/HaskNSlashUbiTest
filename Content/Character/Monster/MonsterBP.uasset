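; Player-controlled monster character with a floaty jump, aimed mid-air smash and dash, driven by gamepad, mouse, or touch and tilt.
; Jump drives gravity from a timeline while a camera trace places the smash target; punching while airborne impulses toward it, with shake on impact.
; Dash briefly hides the mesh during a forward impulse, boosting gravity in air.
; Movement adjusts spring arm length and camera yaw; a debug input spawns AI monsters.
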(event OnComponentHit(CapsuleComponent)
  (params (HitComponent :type Primitive%20Component%20Object%20Reference) (OtherActor :type Actor%20Object%20Reference) (OtherComp :type Primitive%20Component%20Object%20Reference) (NormalImpulse :type Vector :default "0, 0, 0") (Hit :type Hit%20Result%20Structure%20%28by%20ref%29))
  ;[1 0.4803 0.5764] Hide Smash Target on Collision with world static
  (Utilities|FlowControl|Sequence
    (:then_0
      (if (Utilities|Enum|Equal(Enum) (Collision|GetCollisionObjectType (.hitcomponent Hit)) "ECC_WorldStatic")
        (if (Variables|Default|GetIsDashing)
          (Variables|Default|SetIsDashing false))
        (Rendering|SetVisibility (Variables|Default|GetSmashTarget) false false)
        (Variables|/Script/Engine.CharacterMovementComponent|SetGravityScale (Variables|Character|GetCharacterMovement) 1.0)
        (if (Variables|Default|GetIsSmashRotation)
          (Variables|Default|SetIsSmashRotation false)
          (Class|PlayerController|ClientPlayCameraShake (Game|GetPlayerController 0) "/Game/Character/Monster/SmashCameraShake.SmashCameraShake_C" 2.5 "CameraLocal" "0, 0, 0")
          ;;[1 1 1] Spawn "Explosion" emitter
          (Effects|SpawnEmitteratLocation "/Game/StarterContent/Particles/P_Explosion.P_Explosion" (Transformation|GetWorldLocation (Variables|Character|GetMesh)) "0,0.000000, 0"))))
    (:then_1
      (Class|CharacterMovementComponent|CalcVelocity (Variables|Character|GetCharacterMovement) (Variables|Default|GetDeltaSeconds) 5e+03 false 5e+03))))

(event Custom|SmashRotation
  (bind _returnvalue (Transformation|GetActorRotation))
  ;[0.6477 1 0.6747] Smash Rotation
  (Transformation|SetActorRotation (Math|Rotator|MakeRotator (.roll _returnvalue) (.pitch _returnvalue) (Math|Interpolation|FInterpTo (.yaw _returnvalue) (Variables|Default|GetSmashYawRotation) (Variables|Default|GetDeltaSeconds) 2e+01))))

(event Custom|JumpInput
  (bind _smashlocation (Variables|Default|GetSmashLocation))
  (bind _capsulecomponent (Variables|Collision|GetCapsuleComponent))
  (bind _audiocomponent (Variables|Default|GetAudioComponent))
  (bind _returnvalue (Transformation|GetWorldLocation _capsulecomponent))
  (bind _returnvalue_2 (- _smashlocation _returnvalue))
  ;[0.4045 1 0.5939] Smash Punch
  ;;[1 1 1] If Pressed while IsInAir
  (if (AI|Components|NavMovement|IsFalling (Variables|Character|GetCharacterMovement))
    ;;[1 1 1] If we have a valid Smash location
    (if (Variables|Default|GetIsSmashLocationValid)
      ;;[1 1 1] Then Impulse at SmashStrength to SmashLocation
      (Physics|AddImpulse (Variables|Character|GetCharacterMovement) (* _returnvalue_2 (Variables|Default|GetSmashStrength)) true)
      (Variables|Default|SetIsSmashRotation true)
      (Variables|Default|SetSmashYawRotation (.yaw (Math|Conversions|RotationFromXVector _returnvalue_2)))
      ;;[1 1 1] Spawn "Explosion" emitter
      (Effects|SpawnEmitteratLocation "/Game/StarterContent/Particles/P_Explosion.P_Explosion" (Transformation|GetWorldLocation (Variables|Character|GetMesh)) "0,0.000000,0.000000")
      (Audio|Components|Audio|Stop (Variables|Default|GetAudioComponent))
      (Audio|Components|Audio|SetSound _audiocomponent "/Game/StarterContent/Audio/Collapse02.Collapse02")
      (Audio|Components|Audio|Play _audiocomponent 0.2)
      (Utilities|FlowControl|Delay 0.75)
      (Audio|Components|Audio|Stop _audiocomponent))))

(event Custom|TouchReleased
  (params (Location :type Vector) (Finger%20Index :type ETouchIndex%20Enum))
  ;[0.5261 0 1] MOBILE : Jump input and setting if joystick is in use
  (if (and (Variables|Default|GetJoystickInUse) (Utilities|Enum|Equal(Enum) Finger%20Index "Touch1"))
    (Variables|Default|SetJoystickInUse false)))

(event Custom|TouchPressed
  (params (Location :type Vector) (Finger%20Index :type ETouchIndex%20Enum))
  (bind _returnvalue (Game|GetPlayerController 0))
  (bind _mesh (Variables|Character|GetMesh))
  (bind _mesh_2 (Variables|Character|GetMesh))
  (bind _mesh_3 (Variables|Character|GetMesh))
  (bind _camerachar (Variables|Default|GetCameraChar))
  (bind _smashmaxrange (Variables|Default|GetSmashMaxRange))
  (bind _returnvalue_2 (Transformation|GetWorldLocation _mesh_2))
  (bind _returnvalue_3 (Math|Vector|GetForwardVector _camerachar))
  (bind _returnvalue_4 (Transformation|GetWorldLocation _mesh))
  (bind (_sizex _sizey) (HUD|GetViewportSize _returnvalue))
  (bind _returnvalue_5 (Transformation|GetWorldLocation _mesh_3))
  (bind (_x _y) (Math|Vector|BreakVector _returnvalue_4))
  (bind _returnvalue_6 (Math|Vector|Normalize _returnvalue_3))
  (bind _returnvalue_7 (* _returnvalue_6 _smashmaxrange))
  (bind _output_get (Variables|Default|SetTouchLocation Location))
  ;[0.5261 0 1] MOBILE : Jump input and setting if joystick is in use
  (Development|PrintString (Utilities|String|ToString(Boolean) (and (< (.x _output_get) (Math|Conversions|ToFloat(Integer) (/ _sizex 4))) (> (.y _output_get) (* (/ _sizey 4) 3.0)))))
  (if (Variables|Default|GetJoystickInUse)
    _
    (else
      (Variables|Default|SetJoystickInUse (and (< (.x _output_get) (Math|Conversions|ToFloat(Integer) (/ _sizex 4))) (> (.y _output_get) (* (/ _sizey 4) 3.0))))))
  (if (Variables|Default|GetJoystickInUse)
    (if (Utilities|Enum|Equal(Enum) Finger%20Index "Touch2")
      (if (and (< (.x _output_get) (Math|Conversions|ToFloat(Integer) (/ _sizex 4))) (> (.y _output_get) (* (/ _sizey 4) 3.0)))
        (CallFunction|SpawnEnemyMobile)
        (else
          ;[1 0.4674 0.9142] Jump State and Smash Location management
          (if (and (not (Variables|Default|GetIsDashing)) (not (Variables|Default|GetIsSmashRotation))) :!label _label
            ;;[1 1 1] Reset SmashLocationValid
            (Variables|Default|SetIsSmashLocationValid false)
            (Character|Jump)
            ;;[1 1 1] Display Smash Target
            (Rendering|SetVisibility (Variables|Default|GetSmashTarget) true false)
            ;;[1 1 1] Edit Gravity Scale to have a "flying jump"
            (bind _jumpgravity (Timeline|Gravity%20Scale%20Curve PlayFromStart)
              (:Update
                (if (Variables|Default|GetIsDashing)
                  (Timeline|Gravity%20Scale%20Curve Stop)
                  (else
                    (Variables|/Script/Engine.CharacterMovementComponent|SetGravityScale (Variables|Character|GetCharacterMovement) _jumpgravity)
                    ;;[1 1 1] Raycast from Character to CameraForward*1000
                    (bind (_outhit _returnvalue_8) (Collision|LineTraceForObjects _returnvalue_5 (+ _returnvalue_5 (* (Math|Vector|GetForwardVector (Variables|Default|GetCameraChar)) 2.5e+03)) (Utilities|Array|MakeArray "ObjectTypeQuery1") false 0 "None"))
                    ;;[1 1 1] If HIT and HitDistance < SmashMaxRange
                    (if (and _returnvalue_8 (< (Math|Vector|VectorLength (- (Math|Vector|MakeVector (.X (Math|Vector|BreakVector (.Location (Collision|BreakHitResult _outhit)))) (.Y (Math|Vector|BreakVector (.Location (Collision|BreakHitResult _outhit)))) 0.0) (Math|Vector|MakeVector (.x _returnvalue_2) (.y _returnvalue_2) 0.0))) (Variables|Default|GetSmashMaxRange)))
                      ;;[1 1 1] SmashLocation is the HitPoint and location is valid
                      (bind _output_get_2 (Variables|Default|SetSmashLocation (.Location (Collision|BreakHitResult _outhit))))
                      (Transformation|SetWorldLocation (Variables|Default|GetSmashTarget) _output_get_2 false false)
                      (Variables|Default|SetIsSmashLocationValid true)
                      (else
                        ;;[1 1 1] SmashLocation maximal range position
                        (bind _output_get_3 (Variables|Default|SetSmashLocation (+ (Math|Vector|MakeVector _x _y 0.0) (Math|Vector|MakeVector (.x _returnvalue_7) (.y _returnvalue_7) 32.0))))
                        (Transformation|SetWorldLocation (Variables|Default|GetSmashTarget) _output_get_3 false false)
                        (Variables|Default|SetIsSmashLocationValid true)))))))))))
    (elif (Utilities|Enum|Equal(Enum) Finger%20Index "Touch1")
      (goto _label))))

(event Custom|SpawnEnemyMobile
  ;[1 1 1] ROCKET JUMP // Spawn Enemy
  (bind _returnvalue (AI|SpawnAIFromClass "/Game/AI/AI_MonsterBasic.AI_MonsterBasic_C" 0 (Math|Vector|MakeVector (Math|Random|RandomFloatinRange 2.3e+02 3.652e+04) (Math|Random|RandomFloatinRange 0.0 3.515e+04) 9e+01) "0, 0, 0" false))
  (bind _asai_monster_basic (Utilities|Casting|CastToAI_MonsterBasic _returnvalue))
  (Default|Activate _asai_monster_basic))

(event EventTick
  (params (DeltaSeconds :type Float%20%28single-precision%29))
  (bind _returnvalue (Transformation|GetVelocity))
  (bind _charactermovement (Variables|Character|GetCharacterMovement))
  (bind _charactermovement_2 (Variables|Character|GetCharacterMovement))
  (bind _returnvalue_2 (AI|Components|NavMovement|IsFalling _charactermovement))
  (bind _returnvalue_3 (Math|Vector|VectorLength _returnvalue))
  (bind _returnvalue_4 (> _returnvalue_3 3e+03))
  (bind _returnvalue_5 (and _returnvalue_4 _returnvalue_2))
  (Variables|Default|SetDeltaSeconds DeltaSeconds)
  (Utilities|FlowControl|Sequence
    (:then_0
      (if (Variables|Default|GetIsSmashRotation)
        (CallFunction|SmashRotation)))
    (:then_1
      (if _returnvalue_5
        (Utilities|FlowControl|DoOnce false :!label _label
          (:Completed
            (Utilities|FlowControl|Delay 0.2)
            (if _returnvalue_5
              (Variables|/Script/Engine.CharacterMovementComponent|SetGravityScale _charactermovement_2 (+ (Variables|/Script/Engine.CharacterMovementComponent|GetGravityScale _charactermovement_2) 1e+02))
              (Utilities|FlowControl|Sequence
                (:then_0
                  (goto _label Reset))
                (:then_1
                  (Utilities|FlowControl|Delay 0.2)
                  (Variables|/Script/Engine.CharacterMovementComponent|SetGravityScale _charactermovement_2 1.0)
                  (goto _label Reset)))
              (else
                (goto _label Reset)))))))))

(event Input|ActionEvents|InputActionDash
  (params (Key :type Key%20Structure :default "AnyKey"))
  (bind _charactermovement (Variables|Character|GetCharacterMovement))
  (bind _audiocomponent (Variables|Default|GetAudioComponent))
  ;[0 0.6274 1] Dash
  (:Pressed
    (if (AI|Components|NavMovement|IsFalling (Variables|Character|GetCharacterMovement))
      (if (not (Variables|Default|GetIsDashing))
        (Variables|Default|SetIsDashing true :!label _label)
        (Utilities|FlowControl|Sequence
          (:then_0
            ;;[1 1 1] Spawn "Explosion" emitter
            (Effects|SpawnEmitteratLocation "/Game/StarterContent/Particles/P_ExplosionBlue.P_ExplosionBlue" (Transformation|GetWorldLocation (Variables|Character|GetMesh)) "0,0.000000, 0")
            ;;[1 1 1] Activate Trail FX
            (Components|Activation|Activate (Variables|Default|GetVanishParticle) true)
            (Utilities|FlowControl|Delay 0.1)
            ;;[1 1 1] Hide Mesh
            (Rendering|SetVisibility (Variables|Character|GetMesh) false false)
            ;;[1 1 1] Impulse player forward at DashStrength
            (Physics|AddImpulse (Variables|Character|GetCharacterMovement) (* (Math|Vector|GetForwardVector (Variables|Collision|GetCapsuleComponent)) (Variables|Default|GetDashStrength)) true)
            (Utilities|FlowControl|Sequence
              (:then_0
                ;;[1 1 1] If Player IsInAir, increase GravityScale for a while to avoid Infinite Impulse due to no ground friction as we're InTheAir
                (if (AI|Components|NavMovement|IsFalling _charactermovement)
                  (Variables|/Script/Engine.CharacterMovementComponent|SetGravityScale _charactermovement (+ (Variables|/Script/Engine.CharacterMovementComponent|GetGravityScale _charactermovement) 1e+02))
                  (Utilities|FlowControl|Delay 0.5)
                  (Variables|/Script/Engine.CharacterMovementComponent|SetGravityScale _charactermovement 1.0)
                  (if (not (AI|Components|NavMovement|IsFalling (Variables|Character|GetCharacterMovement))) :!label _label_2
                    (Variables|Default|SetIsDashing false))))
              (:then_1
                (Utilities|FlowControl|Delay 0.2)
                ;;[1 1 1] Show Mesh
                (Rendering|SetVisibility (Variables|Character|GetMesh) true false)
                ;;[1 1 1] Spawn "Explosion" Emitter
                (Effects|SpawnEmitteratLocation "/Game/StarterContent/Particles/P_ExplosionBlue.P_ExplosionBlue" (Transformation|GetWorldLocation (Variables|Character|GetMesh)) "0,0.000000, 0")
                (Utilities|FlowControl|Delay 0.1)
                ;;[1 1 1] Deactivate Trail
                (Components|Activation|Deactivate (Variables|Default|GetVanishParticle))
                (goto _label_2))))
          (:then_1
            (Audio|Components|Audio|SetSound _audiocomponent "/Game/StarterContent/Audio/Steam01.Steam01")
            (Audio|Components|Audio|Play _audiocomponent 0.2)
            (Utilities|FlowControl|Delay 0.6)
            (Audio|Components|Audio|Stop _audiocomponent))))
      (else
        (goto _label)))))

(event Input|ActionEvents|InputActionRocketJump
  (params (Key :type Key%20Structure :default "AnyKey"))
  ;[1 1 1] ROCKET JUMP // Spawn Enemy
  (:Pressed
    (bind _returnvalue (AI|SpawnAIFromClass "/Game/AI/AI_MonsterBasic.AI_MonsterBasic_C" 0 (Math|Vector|MakeVector (Math|Random|RandomFloatinRange 2.3e+02 3.652e+04) (Math|Random|RandomFloatinRange 0.0 3.515e+04) 9e+01) "0, 0, 0" false))
    (bind _asai_monster_basic (Utilities|Casting|CastToAI_MonsterBasic _returnvalue))
    (Default|Activate _asai_monster_basic)))

(event Input|ActionEvents|InputActionJump
  (params (Key :type Key%20Structure :default "AnyKey"))
  (bind _mesh (Variables|Character|GetMesh))
  (bind _mesh_2 (Variables|Character|GetMesh))
  (bind _mesh_3 (Variables|Character|GetMesh))
  (bind _camerachar (Variables|Default|GetCameraChar))
  (bind _smashmaxrange (Variables|Default|GetSmashMaxRange))
  (bind _returnvalue (Transformation|GetWorldLocation _mesh_2))
  (bind _returnvalue_2 (Math|Vector|GetForwardVector _camerachar))
  (bind _returnvalue_3 (Transformation|GetWorldLocation _mesh))
  (bind _returnvalue_4 (Transformation|GetWorldLocation _mesh_3))
  (bind (_x _y) (Math|Vector|BreakVector _returnvalue_3))
  (bind _returnvalue_5 (Math|Vector|Normalize _returnvalue_2))
  (bind _returnvalue_6 (* _returnvalue_5 _smashmaxrange))
  ;[1 0.4674 0.9142] Jump State and Smash Location management
  (:Pressed
    (CallFunction|JumpInput)
    (if (and (not (Variables|Default|GetIsDashing)) (not (Variables|Default|GetIsSmashRotation)))
      ;;[1 1 1] Reset SmashLocationValid
      (Variables|Default|SetIsSmashLocationValid false)
      (Character|Jump)
      ;;[1 1 1] Display Smash Target
      (Rendering|SetVisibility (Variables|Default|GetSmashTarget) true false)
      ;;[1 1 1] Edit Gravity Scale to have a "flying jump"
      (bind _jumpgravity (Timeline|Gravity%20Scale%20Curve PlayFromStart)
        (:Update
          (if (Variables|Default|GetIsDashing)
            (Timeline|Gravity%20Scale%20Curve Stop)
            (else
              (Variables|/Script/Engine.CharacterMovementComponent|SetGravityScale (Variables|Character|GetCharacterMovement) _jumpgravity)
              ;;[1 1 1] Raycast from Character to CameraForward*1000
              (bind (_outhit _returnvalue_7) (Collision|LineTraceForObjects _returnvalue_4 (+ _returnvalue_4 (* (Math|Vector|GetForwardVector (Variables|Default|GetCameraChar)) 2.5e+03)) (Utilities|Array|MakeArray "ObjectTypeQuery1") false 0 "None"))
              ;;[1 1 1] If HIT and HitDistance < SmashMaxRange
              (if (and _returnvalue_7 (< (Math|Vector|VectorLength (- (Math|Vector|MakeVector (.X (Math|Vector|BreakVector (.Location (Collision|BreakHitResult _outhit)))) (.Y (Math|Vector|BreakVector (.Location (Collision|BreakHitResult _outhit)))) 0.0) (Math|Vector|MakeVector (.x _returnvalue) (.y _returnvalue) 0.0))) (Variables|Default|GetSmashMaxRange)))
                ;;[1 1 1] SmashLocation is the HitPoint and location is valid
                (bind _output_get (Variables|Default|SetSmashLocation (.Location (Collision|BreakHitResult _outhit))))
                (Transformation|SetWorldLocation (Variables|Default|GetSmashTarget) _output_get false false)
                (Variables|Default|SetIsSmashLocationValid true)
                (else
                  ;;[1 1 1] SmashLocation maximal range position
                  (bind _output_get_2 (Variables|Default|SetSmashLocation (+ (Math|Vector|MakeVector _x _y 0.0) (Math|Vector|MakeVector (.x _returnvalue_6) (.y _returnvalue_6) 32.0))))
                  (Transformation|SetWorldLocation (Variables|Default|GetSmashTarget) _output_get_2 false false)
                  (Variables|Default|SetIsSmashLocationValid true))))))))))

(event Input|ActionEvents|InputActionPunch
  (params (Key :type Key%20Structure :default "AnyKey"))
  (bind _audiocomponent (Variables|Default|GetAudioComponent))
  (bind _smashlocation (Variables|Default|GetSmashLocation))
  (bind _capsulecomponent (Variables|Collision|GetCapsuleComponent))
  (bind _audiocomponent_2 (Variables|Default|GetAudioComponent))
  (bind _returnvalue (Transformation|GetWorldLocation _capsulecomponent))
  (bind _returnvalue_2 (- _smashlocation _returnvalue))
  ;[0.06939 1 0] Punching
  (:Pressed
    (Variables|Default|SetIsPunching true)
    (Audio|Components|Audio|SetSound _audiocomponent "/Game/StarterContent/Audio/Starter_Birds01.Starter_Birds01")
    (Audio|Components|Audio|Play _audiocomponent 0.0)
    ;[0.4045 1 0.5939] Smash Punch
    ;;[1 1 1] If Pressed while IsInAir
    (if (AI|Components|NavMovement|IsFalling (Variables|Character|GetCharacterMovement))
      ;;[1 1 1] If we have a valid Smash location
      (if (Variables|Default|GetIsSmashLocationValid)
        ;;[1 1 1] Then Impulse at SmashStrength to SmashLocation
        (Physics|AddImpulse (Variables|Character|GetCharacterMovement) (* _returnvalue_2 (Variables|Default|GetSmashStrength)) true)
        (Variables|Default|SetIsSmashRotation true)
        (Variables|Default|SetSmashYawRotation (.yaw (Math|Conversions|RotationFromXVector _returnvalue_2)))
        ;;[1 1 1] Spawn "Explosion" emitter
        (Effects|SpawnEmitteratLocation "/Game/StarterContent/Particles/P_Explosion.P_Explosion" (Transformation|GetWorldLocation (Variables|Character|GetMesh)) "0,0.000000,0.000000")
        (Audio|Components|Audio|Stop _audiocomponent)
        (Audio|Components|Audio|SetSound _audiocomponent_2 "/Game/StarterContent/Audio/Collapse02.Collapse02")
        (Audio|Components|Audio|Play _audiocomponent_2 0.2)
        (Utilities|FlowControl|Delay 0.75)
        (Audio|Components|Audio|Stop _audiocomponent_2))))
  (:Released
    (Variables|Default|SetIsPunching false)))

(event Input|AxisEvents|InputAxisTurn
  (params (AxisValue :type Float%20%28single-precision%29))
  ;[1 1 1] Mouse Control
  (Pawn|Input|AddControllerYawInput AxisValue))

(event Input|AxisEvents|InputAxisTurnRate
  (params (AxisValue :type Float%20%28single-precision%29))
  ;[1 1 1] Gamepad Controls for the camera
  (Pawn|Input|AddControllerYawInput (* AxisValue (Utilities|Time|GetWorldDeltaSeconds) (Variables|Default|GetBaseTurnRate))))

(event Input|AxisEvents|InputAxisLookUpRate
  (params (AxisValue :type Float%20%28single-precision%29))
  (bind _returnvalue (Pawn|GetController))
  (bind _returnvalue_2 (Utilities|Time|GetWorldDeltaSeconds))
  (bind _baselookuprate (Variables|Default|GetBaseLookUpRate))
  (bind _returnvalue_3 (Pawn|GetControlRotation _returnvalue :!class /Script/Engine.Controller))
  (bind _returnvalue_4 (* AxisValue _returnvalue_2 _baselookuprate))
  (bind _returnvalue_5 (> (.pitch _returnvalue_3) 3e+02))
  ;[1 1 1] Gamepad Controls for the camera
  (if (> _returnvalue_4 0.0)
    (if (not (and (< (.pitch _returnvalue_3) 325.0) _returnvalue_5))
      (Pawn|Input|AddControllerPitchInput _returnvalue_4 :!label _label))
    (elif (or _returnvalue_5 (< (.pitch _returnvalue_3) 3e+01))
      (goto _label))))

(event Input|AxisEvents|InputAxisLookUp
  (params (AxisValue :type Float%20%28single-precision%29))
  ;[1 1 1] Mouse Control
  (Pawn|Input|AddControllerPitchInput AxisValue))

(event Input|AxisEvents|InputAxisrotationrate
  (params (AxisValue :type Float%20%28single-precision%29))
  ;[0.5347 0 1] Debug Mobile
)

(event Input|AxisEvents|InputAxistilt
  (params (AxisValue :type Float%20%28single-precision%29))
  ;[0.5347 0 1] Debug Mobile
)

(event Input|AxisEvents|InputAxisacceleration
  (params (AxisValue :type Float%20%28single-precision%29))
  ;[0.5347 0 1] Debug Mobile
)

(event Input|AxisEvents|InputAxisMoveForward
  (params (AxisValue :type Float%20%28single-precision%29))
  (bind _springarm (Variables|Default|GetSpringArm))
  (bind _mesh (Variables|Character|GetMesh))
  (bind _charactermovement (Variables|Character|GetCharacterMovement))
  (bind _returnvalue (AI|Components|NavMovement|IsFalling _charactermovement))
  ;[1 1 1] Movement
  (Pawn|Input|AddMovementInput (* (Math|Vector|GetForwardVector (Variables|Default|GetCameraChar)) 1.0) AxisValue true)
  ;[1 0.9415 0] Are we going backward ? MeshForward.dot.CamToMeshDirection
  (bind _output_get (Variables|Default|SetCamToMeshDirection (Math|Vector|Normalize (- (Transformation|GetWorldLocation _mesh) (Transformation|GetWorldLocation (Variables|Default|GetCameraChar))))))
  (bind _output_get_2 (Variables|Default|SetIsCameraDistantForBackwalk (< (Math|Vector|DotProduct _output_get (Math|Vector|Normalize (Math|Vector|GetRightVector _mesh))) -0.3)))
  (if (or _output_get_2 _returnvalue)
    ;[1 0.9415 0] Interp SpringArm to 800 (backward value) or 600 (jumping value)
    (if _returnvalue
      (Variables|Default|SetBackwardCameraDistance 6e+02)
      (else
        (Variables|Default|SetBackwardCameraDistance 8e+02)))
    (Variables|/Script/Engine.SpringArmComponent|SetTargetArmLength _springarm (Math|Interpolation|FInterpTo (Variables|/Script/Engine.SpringArmComponent|GetTargetArmLength _springarm) (Variables|Default|GetBackwardCameraDistance) (Variables|Default|GetDeltaSeconds) 1.5))
    (else
      ;[1 0.9415 0] Interp SpringArm to 300 (default value)
      (Variables|/Script/Engine.SpringArmComponent|SetTargetArmLength (Variables|Default|GetSpringArm) (Math|Interpolation|FInterpTo (Variables|/Script/Engine.SpringArmComponent|GetTargetArmLength (Variables|Default|GetSpringArm)) 3e+02 (Variables|Default|GetDeltaSeconds) 1.5)))))

(event Input|AxisEvents|InputAxisMoveRight
  (params (AxisValue :type Float%20%28single-precision%29))
  (bind _camerachar (Variables|Default|GetCameraChar))
  (bind _relativerotation (Variables|/Script/Engine.SceneComponent|GetRelativeRotation _camerachar))
  ;[1 1 1] Movement
  (Pawn|Input|AddMovementInput (* (Math|Vector|GetRightVector (Variables|Default|GetCameraChar)) 1.0) AxisValue true)
  ;[1 0.9415 0] Camera Rotation Interp
  (Variables|Default|SetHorizontalDirectionFromCamera (Math|Vector|DotProduct (Math|Vector|Normalize (Math|Vector|GetForwardVector (Variables|Character|GetMesh))) (Variables|Default|GetCamToMeshDirection)))
  (Transformation|SetRelativeRotation _camerachar (Math|Rotator|MakeRotator (.roll _relativerotation) (.pitch _relativerotation) (Math|Interpolation|FInterpTo (.yaw _relativerotation) (* (Math|Curves|GetFloatValue (Variables|Default|GetRotationCurve) (Variables|Default|GetHorizontalDirectionFromCamera)) (Variables|Default|GetCameraSideRotationMax)) (Variables|Default|GetDeltaSeconds) 3.0)) false false))

(event Input|TouchEvents|InputTouch
  (params (Location :type Vector) (FingerIndex :type ETouchIndex%20Enum))
  (bind _audiocomponent (Variables|Default|GetAudioComponent))
  (bind _smashlocation (Variables|Default|GetSmashLocation))
  (bind _capsulecomponent (Variables|Collision|GetCapsuleComponent))
  (bind _audiocomponent_2 (Variables|Default|GetAudioComponent))
  (bind _returnvalue (Transformation|GetWorldLocation _capsulecomponent))
  (bind _returnvalue_2 (- _smashlocation _returnvalue))
  ;[0.5166 0 1] MOBILE : Touch for smash depending on Joystick use or not
  (:Pressed
    (CallFunction|TouchPressed Location FingerIndex)
    (if (Variables|Default|GetJoystickInUse)
      (if (Utilities|Enum|Equal(Enum) FingerIndex "Touch4")
        ;[0.06939 1 0] Punching
        (Variables|Default|SetIsPunching true :!label _label)
        (Audio|Components|Audio|SetSound _audiocomponent "/Game/StarterContent/Audio/Starter_Birds01.Starter_Birds01")
        (Audio|Components|Audio|Play _audiocomponent 0.0)
        ;[0.4045 1 0.5939] Smash Punch
        ;;[1 1 1] If Pressed while IsInAir
        (if (AI|Components|NavMovement|IsFalling (Variables|Character|GetCharacterMovement))
          ;;[1 1 1] If we have a valid Smash location
          (if (Variables|Default|GetIsSmashLocationValid)
            ;;[1 1 1] Then Impulse at SmashStrength to SmashLocation
            (Physics|AddImpulse (Variables|Character|GetCharacterMovement) (* _returnvalue_2 (Variables|Default|GetSmashStrength)) true)
            (Variables|Default|SetIsSmashRotation true)
            (Variables|Default|SetSmashYawRotation (.yaw (Math|Conversions|RotationFromXVector _returnvalue_2)))
            ;;[1 1 1] Spawn "Explosion" emitter
            (Effects|SpawnEmitteratLocation "/Game/StarterContent/Particles/P_Explosion.P_Explosion" (Transformation|GetWorldLocation (Variables|Character|GetMesh)) "0,0.000000,0.000000")
            (Audio|Components|Audio|Stop _audiocomponent)
            (Audio|Components|Audio|SetSound _audiocomponent_2 "/Game/StarterContent/Audio/Collapse02.Collapse02")
            (Audio|Components|Audio|Play _audiocomponent_2 0.2)
            (Utilities|FlowControl|Delay 0.75)
            (Audio|Components|Audio|Stop _audiocomponent_2))))
      (elif (Utilities|Enum|Equal(Enum) FingerIndex "Touch3")
        (goto _label))))
  (:Released
    (CallFunction|TouchReleased Location FingerIndex)
    (if (Variables|Default|GetJoystickInUse)
      (if (Utilities|Enum|Equal(Enum) FingerIndex "Touch3")
        (Variables|Default|SetIsPunching false :!label _label_2))
      (elif (Utilities|Enum|Equal(Enum) FingerIndex "Touch3")
        (goto _label_2)))))

(event Input|TouchEvents|InputTouch
  (params (Location :type Vector) (FingerIndex :type ETouchIndex%20Enum))
  (bind _charactermovement (Variables|Character|GetCharacterMovement))
  (bind _audiocomponent (Variables|Default|GetAudioComponent))
  ;[0.5815 0 1] Comment
  (:Pressed
    (if (Variables|Default|GetJoystickInUse)
      (if (Utilities|Enum|Equal(Enum) FingerIndex "Touch3")
        ;[0 0.6274 1] Dash
        (if (AI|Components|NavMovement|IsFalling (Variables|Character|GetCharacterMovement)) :!label _label
          (if (not (Variables|Default|GetIsDashing))
            (Variables|Default|SetIsDashing true :!label _label_2)
            (Utilities|FlowControl|Sequence
              (:then_0
                ;;[1 1 1] Spawn "Explosion" emitter
                (Effects|SpawnEmitteratLocation "/Game/StarterContent/Particles/P_ExplosionBlue.P_ExplosionBlue" (Transformation|GetWorldLocation (Variables|Character|GetMesh)) "0,0.000000, 0")
                ;;[1 1 1] Activate Trail FX
                (Components|Activation|Activate (Variables|Default|GetVanishParticle) true)
                (Utilities|FlowControl|Delay 0.1)
                ;;[1 1 1] Hide Mesh
                (Rendering|SetVisibility (Variables|Character|GetMesh) false false)
                ;;[1 1 1] Impulse player forward at DashStrength
                (Physics|AddImpulse (Variables|Character|GetCharacterMovement) (* (Math|Vector|GetForwardVector (Variables|Collision|GetCapsuleComponent)) (Variables|Default|GetDashStrength)) true)
                (Utilities|FlowControl|Sequence
                  (:then_0
                    ;;[1 1 1] If Player IsInAir, increase GravityScale for a while to avoid Infinite Impulse due to no ground friction as we're InTheAir
                    (if (AI|Components|NavMovement|IsFalling _charactermovement)
                      (Variables|/Script/Engine.CharacterMovementComponent|SetGravityScale _charactermovement (+ (Variables|/Script/Engine.CharacterMovementComponent|GetGravityScale _charactermovement) 1e+02))
                      (Utilities|FlowControl|Delay 0.5)
                      (Variables|/Script/Engine.CharacterMovementComponent|SetGravityScale _charactermovement 1.0)
                      (if (not (AI|Components|NavMovement|IsFalling (Variables|Character|GetCharacterMovement))) :!label _label_3
                        (Variables|Default|SetIsDashing false))))
                  (:then_1
                    (Utilities|FlowControl|Delay 0.2)
                    ;;[1 1 1] Show Mesh
                    (Rendering|SetVisibility (Variables|Character|GetMesh) true false)
                    ;;[1 1 1] Spawn "Explosion" Emitter
                    (Effects|SpawnEmitteratLocation "/Game/StarterContent/Particles/P_ExplosionBlue.P_ExplosionBlue" (Transformation|GetWorldLocation (Variables|Character|GetMesh)) "0,0.000000, 0")
                    (Utilities|FlowControl|Delay 0.1)
                    ;;[1 1 1] Deactivate Trail
                    (Components|Activation|Deactivate (Variables|Default|GetVanishParticle))
                    (goto _label_3))))
              (:then_1
                (Audio|Components|Audio|SetSound _audiocomponent "/Game/StarterContent/Audio/Steam01.Steam01")
                (Audio|Components|Audio|Play _audiocomponent 0.2)
                (Utilities|FlowControl|Delay 0.6)
                (Audio|Components|Audio|Stop _audiocomponent))))
          (else
            (goto _label_2))))
      (elif (Utilities|Enum|Equal(Enum) FingerIndex "Touch2")
        (goto _label)))))

(event Input|KeyboardEvents|Gravity
  (params (AxisValue :type Vector))
  (bind _y (Math|Vector|BreakVector AxisValue))
  (bind _mobilehorizontalsensibility (Variables|Default|GetMobileHorizontalSensibility))
  (bind _returnvalue (/ _y _mobilehorizontalsensibility))
  ;[0.4335 0 1] MOBILE Tilt : get a Delta tilt to turn a bit the camera when tilting -> should have a continuous rotation above a certain rate
  (Development|PrintString (Utilities|String|ToString(Float) _returnvalue) true true "(R=0.000000,G=1.000000,B=0.178514,A=1.000000)" 0.0)
  (Pawn|Input|AddControllerYawInput (- _returnvalue (Variables|Default|GetMobileHorizontalInput)))
  (Variables|Default|SetMobileHorizontalInput _returnvalue))

(fn ConstructionScript)