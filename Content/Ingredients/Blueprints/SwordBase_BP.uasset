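; Sword base actor that fills with power and spawns a SwordPickup_BP above itself once full.
; BeginPlay creates an off-screen indicator widget, and Tick feeds it current power over max power as completion, with a DoOnce guarding the spawn at a fixed height.
; Activation trigger overlaps show or hide the indicator until a shutdown event marks the sword as taken.
; An older gauge-update and face-player chain is left unconnected.
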(event EventBeginPlay
  (bind _returnvalue (UserInterface|CreateWidget "/Game/UI/OffScreen_Widget.OffScreen_Widget_C" 0 self))
  (bind _output_get (Variables|Default|SetPositionIndicator _returnvalue))
  (UserInterface|Viewport|AddtoViewport _output_get 0))

(event Collision|EventActorBeginOverlap
  (params (OtherActor :type Actor%20Object%20Reference)))

(event EventShutdownPositionIndicator
  (bind _positionindicator (Variables|Default|GetPositionIndicator))
  (Default|SetActive _positionindicator false)
  (Variables|/Game/UI/OffScreen_Widget.OffScreen_Widget_C|SetSwordTaken _positionindicator true))

(event EventActivationTriggerBoxOverlapBegin
  (bind _positionindicator (Variables|Default|GetPositionIndicator))
  (if (not (Variables|/Game/UI/OffScreen_Widget.OffScreen_Widget_C|GetSwordTaken _positionindicator))
    (Default|SetActive _positionindicator true)))

(event EventActivationTriggerBoxOverlapEnd
  (Default|SetActive (Variables|Default|GetPositionIndicator) false))

(event EventTick
  (params (DeltaSeconds :type Float%20%28single-precision%29))
  (bind _returnvalue (Transformation|GetActorTransform))
  (bind _output_get (Variables|/Game/UI/OffScreen_Widget.OffScreen_Widget_C|SetCompletionPercentage (Variables|Default|GetPositionIndicator) (/ (Class|NDUSwordBase|GetCurrentPower) (Variables|Default|GetMaxPower))))
  (if (>= _output_get 1.0)
    (Utilities|FlowControl|DoOnce false
      (:Completed
        (Game|SpawnActorfromClass "/Game/Ingredients/Blueprints/SwordPickup_BP.SwordPickup_BP_C" (Math|Transform|MakeTransform (Math|Vector|MakeVector (.x (.location _returnvalue)) (.y (.location _returnvalue)) 2.1e+02) (Math|Rotator|MakeRotator 0.0 3e+01 0.0) (.scale _returnvalue)) "AlwaysSpawn" 0 0)))))

(fn ConstructionScript)