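; Battery pickup that sends power to the player's sword base when collected.
; WasCollected plays an explosion, knocks the mesh up and away from the player, then hides it.
; If the linked sword base is active, a timeline lerps a spark emitter to the player's base and adds power once partway through, then calls parent collection logic.
; Otherwise it finishes after a delay; Tick keeps the player's base reference current.
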(event EventBeginPlay)

(event Collision|EventActorBeginOverlap
  (params (OtherActor :type Actor%20Object%20Reference)))

(event EventTick
  (params (DeltaSeconds :type Float%20%28single-precision%29))
  (bind _ashack_nslash_character (Utilities|Casting|CastToHackNSlashCharacter (Game|GetPlayerCharacter 0)))
  (Utilities|IsValid (Class|HackNSlashCharacter|GetCurrentSwordBase _ashack_nslash_character)
    (:Is%20Valid
      (Variables|Default|SetPlayerBase (Class|HackNSlashCharacter|GetCurrentSwordBase _ashack_nslash_character)))))

(event EventWasCollected
  (bind _returnvalue (Transformation|GetActorLocation))
  (bind _returnvalue_2 (Game|GetPlayerCharacter 0))
  (bind _returnvalue_3 (Transformation|GetActorLocation _returnvalue_2))
  (bind _returnvalue_4 (Math|Vector2D|MakeVector2D (.x _returnvalue) (.y _returnvalue)))
  (bind _returnvalue_5 (Math|Vector2D|MakeVector2D (.x _returnvalue_3) (.y _returnvalue_3)))
  (bind _returnvalue_6 (- _returnvalue_4 _returnvalue_5))
  (bind _ashack_nslash_character (Utilities|Casting|CastToHackNSlashCharacter (Game|GetPlayerCharacter 0))
    (:then
      _)
    (:CastFailed
      (Development|PrintString "Hello")))
  (Variables|Default|SetTargetBaseLocation (Transformation|GetWorldLocation (Variables|/Script/HackNSlash.NDU_SwordBase|GetBaseMesh (Class|HackNSlashCharacter|GetCurrentSwordBase _ashack_nslash_character))))
  (Effects|SpawnEmitterAttached "/Game/StarterContent/Particles/P_Explosion.P_Explosion" (Variables|Default|GetPickupMesh) "None" "0, 0, 0" "0, 0, 0" "SnapToTargetIncludingScale")
  (Physics|AddImpulse (Variables|Default|GetPickupMesh) (Math|Vector|MakeVector (* (.x _returnvalue_6) 1e+01) (* (.y _returnvalue_6) 1e+01) 5e+02) "None" true)
  (Utilities|FlowControl|Sequence
    (:then_0
      (Utilities|FlowControl|Delay 1.0)
      (Rendering|SetVisibility (Variables|Default|GetPickupMesh) false true))
    (:then_1
      (if (Class|NDUSwordBase|IsActive (Class|NDUPickup|GetLinkedSwordBase))
        (bind _returnvalue_7 (Effects|SpawnEmitteratLocation "/Game/StarterContent/Particles/P_Sparks2.P_Sparks2" (Transformation|GetWorldLocation (Variables|Default|GetPickupMesh)) "0, 0,0.000000"))
        (bind _alpha (Timeline|MoveCurve Play)
          (:Update
            (Transformation|SetWorldLocation _returnvalue_7 (Math|Vector|Lerp(Vector) (Transformation|GetWorldLocation _returnvalue_7) (+ (Variables|Default|GetTargetBaseLocation) "0, 0,5.000000") _alpha) false false)
            (if (>= _alpha 0.14)
              (Utilities|FlowControl|DoOnce false
                (:Completed
                  (Class|NDUSwordBase|AddPower (Variables|Default|GetPlayerBase) 1.0)))))
          (:Finished
            (Components|DestroyComponent _returnvalue_7 :!label _label)
            (|CallParentFunction)))
        (else
          (Utilities|FlowControl|Delay 2.0)
          (goto _label))))))

(fn ConstructionScript)