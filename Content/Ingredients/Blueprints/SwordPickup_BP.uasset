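; SwordPickup_BP is a sword pickup actor with a glow tied to its lifespan.
; The construction script creates a dynamic material from the pickup mesh's first material and sets a bright initial Emissive.
; LifeSpanChangeEffect sets Emissive from the ratio of current to total lifespan and prints that value to screen.
; BeginPlay, overlap and Tick are empty, so pickup logic is not in this graph.
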(event EventBeginPlay)

(event Collision|EventActorBeginOverlap
  (params (OtherActor :type Actor%20Object%20Reference)))

(event EventTick
  (params (DeltaSeconds :type Float%20%28single-precision%29)))

(event EventLifeSpanChangeEffect
  (bind _returnvalue (Class|NDUSwordPickup|GetCurrentLifeSpan))
  (bind _returnvalue_2 (Class|NDUSwordPickup|GetLifeSpan))
  (bind _returnvalue_3 (/ _returnvalue _returnvalue_2))
  (bind _returnvalue_4 (Math|Float|Lerp 1.0 0.0 _returnvalue_3))
  (bind _returnvalue_5 (- 1.0 _returnvalue_4))
  (Development|PrintString (Utilities|String|ToString(Float) _returnvalue_5))
  (Rendering|Material|SetScalarParameterValue (Variables|Default|GetPowerMaterial) "Emissive" _returnvalue_5 :!class /Script/Engine.MaterialInstanceDynamic))

(fn ConstructionScript
  (bind _pickupmesh (Variables|Default|GetPickupMesh))
  (bind _returnvalue (Rendering|Material|CreateDynamicMaterialInstance _pickupmesh 0 (Utilities|Array|Get(acopy) (Rendering|Material|GetMaterials _pickupmesh)) :!class /Script/Engine.PrimitiveComponent))
  (bind _output_get (Variables|Default|SetPowerMaterial _returnvalue))
  (Rendering|Material|SetScalarParameterValue _output_get "Emissive" 5.0 :!class /Script/Engine.MaterialInstanceDynamic))